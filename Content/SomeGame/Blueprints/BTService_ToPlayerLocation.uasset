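; Behavior Tree service that gives an AI a move target, normally the player's location, through a Blackboard vector key.
; On activation it writes the first player pawn's nav agent location to the key.
; If that pawn is not controlled, it writes a random navigable point near the AI pawn instead.
; It has no tick logic, so the target refreshes only when the service activates.
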(event EventReceiveActivationAI
  (params (OwnerController :type AI%20Controller%20Object%20Reference) (ControlledPawn :type Pawn%20Object%20Reference))
  (if (not (Class|Pawn|IsControlled (Game|Player|GetPlayerPawn 0)))
    ;[1 1 1] random
    (AI|BehaviorTree|SetBlackboardValueasVector (Variables|Default|GetBlackboardKey) (.RandomLocation (Class|NavigationSystemV1|GetRandomPointinNavigableRadius (Transformation|GetActorLocation ControlledPawn) 5e+02 0 0)))
    (else
      (AI|BehaviorTree|SetBlackboardValueasVector (Variables|Default|GetBlackboardKey) (Pawn|GetNavAgentLocation (Game|Player|GetPlayerPawn 0))))))